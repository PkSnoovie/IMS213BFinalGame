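; BP_PuzzleGate is a gate that swings open once enough puzzle items have been collected.
; CollectItem increments a counter and, on reaching MaxItemsCollected, fires OpenDoor a single time through a DoOnce.
; OpenDoor plays a timeline that lerps the door's relative yaw from closed to 120 degrees.
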(event Custom|Open%20Door
  (bind _doorrotation (Timeline|Open%20Door%20Anim Play)
    (:Update
      (Transformation|SetRelativeRotation (Variables|Default|GetDoor) (Math|Rotator|MakeRotator 0.0 0.0 (Math|Float|Lerp 0.0 1.2e+02 _doorrotation)) false false))))

(event Custom|Collect%20Item
  (Math|Integer|IncrementInt (Variables|Default|GetCurrentItemsCollected)
    (:%20%20
      (if (>= (Variables|Default|GetCurrentItemsCollected) (Variables|Default|GetMaxItemsCollected))
        (Utilities|FlowControl|DoOnce false
          (:Completed
            (CallFunction|OpenDoor)))))))

(fn ConstructionScript)