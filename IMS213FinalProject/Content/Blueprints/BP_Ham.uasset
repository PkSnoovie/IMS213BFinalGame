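; BP_Ham is a collectible ham pickup that the third-person character eats by touching it.
; When the character overlaps its trigger, it increments the character's HamsCollected count and plays a 2D eating sound.
; It then calls CollectItem on one BP_PuzzleGate and one BP_3HamGate, both found by class lookup, and destroys itself.
; A separate ActorBeginOverlap handler only casts to the character and does nothing further.
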(event OnComponentBeginOverlap(Trigger)
  (params (OverlappedComponent :type Primitive%20Component%20Object%20Reference) (OtherActor :type Actor%20Object%20Reference) (OtherComp :type Primitive%20Component%20Object%20Reference) (OtherBodyIndex :type Integer) (bFromSweep :type Boolean) (SweepResult :type Hit%20Result%20Structure%20%28by%20ref%29))
  ;[1 1 1] Comment
  (bind _asbp_third_person_character (Utilities|Casting|CastToBP_ThirdPersonCharacter OtherActor))
  (Math|Integer|IncrementInt (Variables|/Game/ThirdPerson/Blueprints/BP_ThirdPersonCharacter.BP_ThirdPersonCharacter_C|GethamsCollected _asbp_third_person_character)
    (:%20%20
      (Audio|PlaySound2D "/Game/Sounds/eatingsound.eatingsound" 1.0 1.0 0.0 0 0)
      (CallFunction|CollectandCheckItems)
      (Actor|DestroyActor))))

(event Custom|Collect%20And%20Check%20Items
  (bind _returnvalue (Actor|GetActorOfClass "/Game/Blueprints/BP_PuzzleGate.BP_PuzzleGate_C"))
  (Default|CollectItem _returnvalue)
  (bind _returnvalue_2 (Actor|GetActorOfClass "/Game/Blueprints/BP_3HamGate.BP_3HamGate_C"))
  (Default|CollectItem _returnvalue_2))

(event Collision|EventActorBeginOverlap
  (params (OtherActor :type Actor%20Object%20Reference))
  (Utilities|Casting|CastToBP_ThirdPersonCharacter OtherActor))

(fn ConstructionScript)